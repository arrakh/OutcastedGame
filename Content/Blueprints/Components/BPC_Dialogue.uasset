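; Dialogue component that steps through a conversation from DT_Dialogues and displays it on the player's HUD, cached shortly after BeginPlay.
; Each TriggerDialogue call shows the current row's speaker and text, then follows NextRowID.
; A DoOnce opens the dialogue at the default row and fires BeginDialogue.
; A trigger after an end row, or CloseDialogue, closes it, fires EndDialogue and resets the DoOnce, though IsInDialogue stays true.
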(event Custom|TriggerDialogue
  (Utilities|FlowControl|Sequence
    (:then_0
      ;[1 1 1] Conversation Init
      (Utilities|FlowControl|DoOnce false :!label _label
        (:Completed
          (Default|OpenDialogue (Variables|Default|GetHUDRef))
          (Variables|Default|SetCurrentDialogueRow (Variables|Default|GetDefaultDialogueRow))
          (Variables|Default|SetisEnd false)
          (Default|CallBeginDialogue)
          (Variables|Default|SetisInDialogue true))))
    (:then_1
      (if (Variables|Default|GetisEnd)
        (Default|CloseDialogue (Variables|Default|GetHUDRef))
        (Variables|Default|SetisInDialogue true)
        (Default|CallEndDialogue)
        (goto _label Reset)
        (else
          (bind _returnvalue (Utilities|GetDataTableRow "/Game/Data/DataTables/DT_Dialogues.DT_Dialogues" (Variables|Default|GetCurrentDialogueRow))
            (:then
              (Default|SetDialogue (Variables|Default|GetHUDRef) (.speakername _returnvalue) (.text _returnvalue))
              (Variables|Default|SetisEnd (.isend _returnvalue))
              (Variables|Default|SetCurrentDialogueRow (.nextrowid _returnvalue)))))))))

(event Custom|CloseDialogue
  (Default|CloseDialogue (Variables|Default|GetHUDRef))
  (Variables|Default|SetisInDialogue true)
  (Default|CallEndDialogue)
  ;[1 1 1] Conversation Init
  (Utilities|FlowControl|DoOnce false) ; enters at Reset
)

(event EventBeginPlay
  (bind _returnvalue (CallFunction|GetPlayer))
  (Utilities|FlowControl|Delay 0.1)
  (Variables|Default|SetHUDRef (Variables|/Game/Blueprints/BP_Player.BP_Player_C|GetHUDRef _returnvalue)))

(event EventTick
  (params (DeltaSeconds :type Float%20%28single-precision%29)))