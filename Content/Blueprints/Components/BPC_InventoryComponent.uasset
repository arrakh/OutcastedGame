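; Inventory component that stores item ID and quantity stacks and owns the player's inventory box widget.
; After a short BeginPlay delay it creates WBP_InventoryBox, places it hidden in BP_Player's HUD, and exposes open-at-position and close events.
; AddItemToInv reads max stack size from DT_ItemList, then tops up the first unfilled matching stack or appends one.
; Overflow is written directly into the following array index, replacing any entry there.
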(event Custom|OpenInventory
  (params (Position :type Vector%202D%20Structure))
  (bind _invboxref (Variables|Default|GetInvBoxRef))
  (Class|UserWidget|SetPositioninViewport _invboxref Position true)
  (Widget|SetVisibility _invboxref "Visible"))

(event Custom|CloseInventory
  (Widget|SetVisibility (Variables|Default|GetInvBoxRef) "Hidden"))

(event EventBeginPlay
  (Utilities|FlowControl|Delay 0.1)
  (bind _returnvalue (UserInterface|CreateWidget "/Game/UI/Inventory/WBP_InventoryBox.WBP_InventoryBox_C" (Game|GetPlayerController 0) self))
  (Variables|Default|SetInvBoxRef _returnvalue)
  (bind _asbp_player (Utilities|Casting|CastToBP_Player (Components|GetOwner))
    (:then
      (bind _output_get (Variables|Default|SetComponentHUDRef (Variables|/Game/Blueprints/BP_Player.BP_Player_C|GetHUDRef _asbp_player)))
      (Default|GetSetWidget _output_get (Variables|Default|GetInvBoxRef) "(X=200.000000,Y=200.000000)")
      (Widget|SetVisibility (Variables|Default|GetInvBoxRef) "Hidden"))
    (:CastFailed
      (Development|PrintString "Player Cast Failed" true true "(R=1.000000,G=0.000000,B=0.009443,A=1.000000)"))))

(event EventTick
  (params (DeltaSeconds :type Float%20%28single-precision%29)))

(fn AddItemtoInv
  (params (ItemID :type Name) (ItemQuantity :type Integer))
  (bind _itemarray (Variables|Default|GetItemArray))
  (bind _output_get (LocalVariables|SetLocalItemID ItemID))
  (LocalVariables|SetLocalItemQuantity ItemQuantity)
  (Development|PrintString (Utilities|String|Append "Adding " (Utilities|String|ToString(Name) (LocalVariables|GetLocalItemID)) " x" (Utilities|String|ToString(Integer) (LocalVariables|GetLocalItemQuantity))) true true "(R=0.000000,G=0.720833,B=0.126304,A=1.000000)")
  (bind _returnvalue (Utilities|GetDataTableRow "/Game/Data/DataTables/DT_ItemList.DT_ItemList" _output_get)
    (:then
      (LocalVariables|Setmaxstack (.maxstacksize _returnvalue))
      (bind (_array_element _array_index) (Utilities|Array|ForEachLoopwithBreak (Variables|Default|GetItemArray) :!label _label)
        (:LoopBody
          (LocalVariables|Setindex _array_index)
          (if (and (Utilities|Name|Equal(Name) (.Item (Utilities|Struct|BreakS_ItemID _array_element)) (LocalVariables|GetLocalItemID)) (!= (.Quantity (Utilities|Struct|BreakS_ItemID _array_element)) (LocalVariables|Getmaxstack)))
            (LocalVariables|SetsameItemFound true)
            (goto _label Break)))
        (:Completed
          (if (LocalVariables|GetsameItemFound)
            (Development|PrintString (Utilities|String|Append "Item Found! Index: " (Utilities|String|ToString(Integer) (LocalVariables|Getindex))) true true "(R=0.353849,G=1.000000,B=0.000000,A=1.000000)")
            (if (> (+ (.quantity (Utilities|Array|Get(acopy) (Variables|Default|GetItemArray) (LocalVariables|Getindex))) (LocalVariables|GetLocalItemQuantity)) (LocalVariables|Getmaxstack))
              ;[0 0 0] Set next index to remainder, fill current index to max stack
              (Utilities|Array|SetArrayElem _itemarray (+ (LocalVariables|Getindex) 1) (Utilities|Struct|MakeS_ItemID (LocalVariables|GetLocalItemID) (- (+ (.quantity (Utilities|Array|Get(acopy) (Variables|Default|GetItemArray) (LocalVariables|Getindex))) (LocalVariables|GetLocalItemQuantity)) (LocalVariables|Getmaxstack))) true)
              (Utilities|Array|SetArrayElem _itemarray (LocalVariables|Getindex) (Utilities|Struct|MakeS_ItemID (LocalVariables|GetLocalItemID) (LocalVariables|Getmaxstack)))
              (Development|PrintString "Exceeding Stack Limit")
              (else
                (Utilities|Array|SetArrayElem _itemarray (LocalVariables|Getindex) (Utilities|Struct|MakeS_ItemID (LocalVariables|GetLocalItemID) (+ (LocalVariables|GetLocalItemQuantity) (.quantity (Utilities|Array|Get(acopy) (Variables|Default|GetItemArray) (LocalVariables|Getindex))))))))
            (else
              (Utilities|Array|Add (Variables|Default|GetItemArray) (Utilities|Struct|MakeS_ItemID (LocalVariables|GetLocalItemID) (LocalVariables|GetLocalItemQuantity)))
              (Development|PrintString "No same item found" true true "(R=1.000000,G=0.042970,B=0.000000,A=1.000000)"))))))
    (:RowNotFound
      (Development|PrintString "Item Not Found" true true "(R=1.000000,G=0.043071,B=0.000000,A=1.000000)"))))