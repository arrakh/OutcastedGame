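; Shop component that opens and closes the shop screen and is set up to handle buying and selling.
; BeginPlay caches the player character as BP_Player.
; ToggleShop removes the screen if its reference is valid, without clearing that reference, otherwise creates WBP_ShopScreen with itself passed in.
; BuyItem and SellItem are empty stubs, and ShopInventory is not yet used.
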(event Custom|ToggleShop
  (bind _shopuiref (Variables|Default|GetShopUIRef)
    (:then
      (Widget|RemovefromParent _shopuiref))
    (:else
      (bind _returnvalue (UserInterface|CreateWidget "/Game/UI/Shop/WBP_ShopScreen.WBP_ShopScreen_C" 0 self))
      (bind _output_get (Variables|Default|SetShopUIRef _returnvalue))
      (UserInterface|Viewport|AddtoViewport _output_get 0)
      (Development|PrintString "Opening shop"))))

(event EventBeginPlay
  (bind _asbp_player (Utilities|Casting|CastToBP_Player (Game|GetPlayerCharacter 0)))
  (Variables|Default|SetPlayerRef _asbp_player))

(fn BuyItem)

(fn SellItem)