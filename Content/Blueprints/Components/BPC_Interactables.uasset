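; Interactable component that outlines its owner's mesh through custom depth and stencil, and relays interaction events.
; On BeginPlay, after a short delay, it caches the owner's skeletal mesh, falling back to static mesh, and applies the overlap stencil color.
; Overlap functions toggle custom depth; StartInteract and EndInteract both apply the interact color.
; Each overlap and interaction call fires a matching event dispatcher.
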(event EventBeginPlay
  (bind _returnvalue (Components|GetOwner))
  (bind _returnvalue_2 (Actor|GetComponentbyClass _returnvalue "/Script/Engine.SkeletalMeshComponent"))
  (Utilities|FlowControl|Delay 0.1)
  (bind _output_get (Variables|Default|SetComponent (select (Utilities|IsValid _returnvalue_2) _returnvalue_2 (Actor|GetComponentbyClass _returnvalue "/Script/Engine.StaticMeshComponent"))))
  (Rendering|SetCustomDepthStencilValue _output_get (.Value (Utilities|Map|Find (Variables|Default|GetOutline) (Variables|Default|GetOverlapColor)))))

(event EventInteract
  (params (PlayerRef :type BP%20Player%20Object%20Reference))
  (Default|CallOnInteract))

(fn EndInteract
  (Rendering|SetCustomDepthStencilValue (Variables|Default|GetComponent) (.Value (Utilities|Map|Find (Variables|Default|GetOutline) (Variables|Default|GetInteractColor))))
  (Default|CallOnEndInteract)
  (return false))

(fn EndOverlap
  (Rendering|SetRenderCustomDepth (Variables|Default|GetComponent) false)
  (Default|CallOnEndOverlap)
  (return false))

(fn StartInteract
  (Rendering|SetCustomDepthStencilValue (Variables|Default|GetComponent) (.Value (Utilities|Map|Find (Variables|Default|GetOutline) (Variables|Default|GetInteractColor))))
  (Default|CallOnStartInteract)
  (return false))

(fn StartOverlap
  (Rendering|SetRenderCustomDepth (Variables|Default|GetComponent) true)
  (Default|CallOnStartOverlap)
  (return false))