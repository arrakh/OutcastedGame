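; Base Blueprint for interactable objects that gives visual highlight feedback through custom depth on ObjectMesh.
; StartOverlap and EndOverlap switch custom depth rendering on and off.
; StartInteract and EndInteract swap the custom depth stencil value to mark the interacting state.
; All four functions return false, and the event graph holds no logic, so calls must come from outside.
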(event EventBeginPlay)

(event Collision|EventActorBeginOverlap
  (params (OtherActor :type Actor%20Object%20Reference)))

(event EventTick
  (params (DeltaSeconds :type Float%20%28single-precision%29)))

(fn ConstructionScript)

(fn EndInteract
  (Rendering|SetCustomDepthStencilValue (Variables|Default|GetObjectMesh) 253)
  (return false))

(fn EndOverlap
  (Rendering|SetRenderCustomDepth (Variables|Default|GetObjectMesh) false)
  (return false))

(fn StartInteract
  (Rendering|SetCustomDepthStencilValue (Variables|Default|GetObjectMesh) 252)
  (return false))

(fn StartOverlap
  (Rendering|SetRenderCustomDepth (Variables|Default|GetObjectMesh) true)
  (return false))