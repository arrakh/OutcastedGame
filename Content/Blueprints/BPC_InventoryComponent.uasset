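; Inventory component that stores item and quantity slots in ItemArray and displays them in a WBP_InventoryBox widget.
; AddItemToInv appends a slot or adds to a found one, but searches by whole struct with quantity zero, so nonzero stacks never match.
; ToggleInventory uses a FlipFlop whose A branch creates, fills and shows the widget from MaxSlot and ItemArray.
; The B branch is unwired, so nothing closes the widget.
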(event Custom|Toggle%20Inventory
  (Utilities|FlowControl|FlipFlop
    (:A
      (bind _returnvalue (UserInterface|CreateWidget "/Game/UI/Inventory/WBP_InventoryBox.WBP_InventoryBox_C" (Game|GetPlayerController 0) (Variables|Default|GetMaxSlot) (Variables|Default|GetItemArray)))
      (Variables|Default|SetInvBoxRef _returnvalue)
      (Default|UpdateSlotContent (Variables|Default|GetInvBoxRef))
      (UserInterface|Viewport|AddtoViewport (Variables|Default|GetInvBoxRef) 0))))

(event Custom|AddItemToInv
  (params (itemName :type Name) (quantity :type Integer))
  (bind _itemarray (Variables|Default|GetItemArray))
  (bind _returnvalue (Utilities|Array|FindItem _itemarray (Utilities|Struct|MakeS_InventorySlot itemName 0)))
  (if (== -1 _returnvalue)
    (Utilities|Array|Add (Variables|Default|GetItemArray) (Utilities|Struct|MakeS_InventorySlot itemName quantity))
    (else
      (Utilities|Array|SetArrayElem (Variables|Default|GetItemArray) _returnvalue (Utilities|Struct|MakeS_InventorySlot itemName (+ quantity (.quantity (Utilities|Array|Get(acopy) _itemarray _returnvalue))))))))

(event EventBeginPlay)

(event EventTick
  (params (DeltaSeconds :type Float%20%28single-precision%29)))