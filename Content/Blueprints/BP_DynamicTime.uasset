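; Day/night cycle actor that advances a game clock and moves the sun to match.
; BeginPlay derives hour length from a configurable day length, starts at noon and starts a looping debug print of the hour.
; While time updates are enabled, Tick advances and wraps the hour, pitches the directional light accordingly, calls UpdateSunDirection and derives the minute.
; The construction script applies the same sun rotation, reflecting the set hour at construction.
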(event Custom|print
  (Development|PrintString (Utilities|String|ToString(Float) (Variables|Default|GetHour))))

(event EventBeginPlay
  (bind _output_get (Variables|Default|SetOneDay (* (Variables|Default|GetDayLengthInMinutes) 6e+01)))
  (Variables|Default|SetOneHour (/ _output_get 24.0))
  (Variables|Default|SetHour 12.0)
  (Utilities|Time|SetTimerbyEvent (delegate Custom|print) 0.1 true))

(event EventTick
  (params (DeltaSeconds :type Float%20%28single-precision%29))
  (bind _directional_light_actor (Variables|Default|GetDirectional%20light%20actor))
  (if (Variables|Default|GetTimeUpdates)
    (if (>= (+ (Variables|Default|GetHour) (/ DeltaSeconds (Variables|Default|GetOneHour))) 24.0)
      (Variables|Default|SetHour 0.0)
      (else
        (Variables|Default|SetHour (+ (Variables|Default|GetHour) (/ DeltaSeconds (Variables|Default|GetOneHour))))))
    (bind _output_get (Variables|Default|SetSunAngle (+ (* (/ (Variables|Default|GetHour) 6.0) 9e+01) 9e+01)))
    (Utilities|IsValid _directional_light_actor
      (:Is%20Valid
        (Transformation|SetActorRotation _directional_light_actor (Math|Rotator|MakeRotator 0.0 _output_get (.yaw (Transformation|GetActorRotation))))
        (CallFunction|UpdateSunDirection)
        (Variables|Default|SetMinute (* 6e+01 (/ (- (Variables|Default|GetHour) (Math|Conversions|ToFloat(Integer) (Math|Float|Truncate (Variables|Default|GetHour)))) 1.0)))))))

(fn ConstructionScript
  (bind _directional_light_actor (Variables|Default|GetDirectional%20light%20actor))
  (|CallParentFunction)
  (bind _output_get (Variables|Default|SetSunAngle (+ (* (/ (Variables|Default|GetHour) 6.0) 9e+01) 9e+01)))
  (Utilities|IsValid _directional_light_actor
    (:Is%20Valid
      (Transformation|SetActorRotation _directional_light_actor (Math|Rotator|MakeRotator 0.0 _output_get (.yaw (Transformation|GetActorRotation))))
      (CallFunction|UpdateSunDirection))))